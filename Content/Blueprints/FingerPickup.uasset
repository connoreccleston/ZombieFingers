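; FingerPickup is an actor Blueprint that continuously spins in place, named as a pickup but containing no collection logic.
; BeginPlay scales the actor up uniformly.
; Each Tick steadily decreases a ZCoord yaw accumulator and constant-rate interpolates the actor's rotation toward that yaw.
; The overlap event is a disabled stub and the construction script is empty.
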(event EventBeginPlay
  (Transformation|SetActorScale3D "2.500000,2.500000,2.500000"))

(event Collision|EventActorBeginOverlap
  (params (OtherActor :type Actor%20Object%20Reference)))

(event EventTick
  (params (DeltaSeconds :type Float%20%28single-precision%29))
  (bind _output_get (Variables|Default|SetZ_Coord (- (Variables|Default|GetZ_Coord) (* DeltaSeconds 25.0))))
  (Transformation|SetActorRotation (Class|KismetMathLibrary|RInterptoConstant (Transformation|GetActorRotation) (Math|Rotator|CombineRotators (Math|Conversions|RotationFromXVector "0, 0, 0") (Math|Rotator|MakeRotator 0.0 0.0 _output_get)) DeltaSeconds 7.5e+02)))

(fn ConstructionScript)