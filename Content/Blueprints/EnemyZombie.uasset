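; Zombie enemy for a twin-stick game that chases the player and hurts it on contact.
; Each tick a debug-drawn Visibility trace runs to the player pawn, with AI MoveTo issued when nothing blocks it and movement stopped otherwise.
; Hitting a TwinStickPawn2 applies damage to it and destroys the zombie.
; Any damage received also destroys the zombie, spawning a FingerPickup at its XY position and a fixed height.
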(event EventBeginPlay)

(event Game|Damage|EventAnyDamage
  (params (Damage :type Float%20%28single-precision%29) (DamageType :type Damage%20Type%20Object%20Reference) (InstigatedBy :type Controller%20Object%20Reference) (DamageCauser :type Actor%20Object%20Reference))
  (bind _returnvalue (Transformation|GetActorLocation))
  (Game|SpawnActorfromClass "/Game/Blueprints/FingerPickup.FingerPickup_C" (Math|Transform|MakeTransform (Math|Vector|MakeVector (.x _returnvalue) (.y _returnvalue) 2.5e+02) "0, 0, 0" "1,1,1") "AlwaysSpawn" 0 0)
  (Actor|DestroyActor))

(event EventTick
  (params (DeltaSeconds :type Float%20%28single-precision%29))
  (bind _returnvalue (Collision|LineTraceByChannel (Transformation|GetActorLocation) (Transformation|GetActorLocation (Game|Player|GetPlayerPawn 0)) "TraceTypeQuery1" false 0 "ForOneFrame")) ; projectiles stop trace
  (if (not _returnvalue)
    (AI|AIMoveTo self "0, 0, 0" (Game|Player|GetPlayerPawn 0) 0.0 false)
    (else
      (AI|Navigation|StopMovement (Pawn|GetController)))))

(event Collision|EventHit
  (params (MyComp :type Primitive%20Component%20Object%20Reference) (Other :type Actor%20Object%20Reference) (OtherComp :type Primitive%20Component%20Object%20Reference) (bSelfMoved :type Boolean) (HitLocation :type Vector :default "0, 0, 0") (HitNormal :type Vector) (NormalImpulse :type Vector :default "0, 0, 0") (Hit :type Hit%20Result%20Structure%20%28by%20ref%29))
  (bind _astwin_stick_pawn_2 (Utilities|Casting|CastToTwinStickPawn2 Other))
  (Game|Damage|ApplyDamage _astwin_stick_pawn_2 1.0 0 0)
  (Actor|DestroyActor))

(fn ConstructionScript)